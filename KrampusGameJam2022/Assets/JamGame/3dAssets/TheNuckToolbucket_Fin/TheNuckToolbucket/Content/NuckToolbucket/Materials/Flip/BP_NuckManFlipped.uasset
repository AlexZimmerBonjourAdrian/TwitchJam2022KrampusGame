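; BP_NuckManFlipped is a player Blueprint whose horizontal movement and look controls can be inverted.
; FlipPlayer sets the IsFlipped flag, and a macro branches on it for the Turn, LookUp and MoveRight axis inputs.
; When flipped, those axis values are negated before driving yaw, pitch and yaw-relative strafing.
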(event EventFlipPlayer
  (params (SetFlip :type Boolean))
  (Variables|Default|SetbIsFlipped SetFlip))

(event Input|AxisEvents|InputAxisTurn
  (params (AxisValue :type Float%20%28single-precision%29))
  (Utilities|IsFlipped
    (:Yes
      (Pawn|Input|AddControllerYawInput (* AxisValue -1.0)))
    (:No
      (Pawn|Input|AddControllerYawInput AxisValue))))

(event Input|AxisEvents|InputAxisLookUp
  (params (AxisValue :type Float%20%28single-precision%29))
  (Utilities|IsFlipped
    (:Yes
      (Pawn|Input|AddControllerPitchInput (* AxisValue -1.0)))
    (:No
      (Pawn|Input|AddControllerPitchInput AxisValue))))

(event Input|AxisEvents|InputAxisMoveRight
  (params (AxisValue :type Float%20%28single-precision%29))
  (bind _returnvalue (Pawn|GetControlRotation :!class /Script/Engine.Pawn))
  (bind _yaw (Math|Rotator|BreakRotator _returnvalue))
  (bind _returnvalue_2 (Math|Rotator|MakeRotator 0.0 0.0 _yaw))
  (bind _returnvalue_3 (Math|Vector|GetRightVector _returnvalue_2))
  (Utilities|IsFlipped
    (:Yes
      (Pawn|Input|AddMovementInput _returnvalue_3 (* AxisValue -1.0) false))
    (:No
      (Pawn|Input|AddMovementInput _returnvalue_3 AxisValue false))))

(fn ConstructionScript
  (|CallParentFunction))