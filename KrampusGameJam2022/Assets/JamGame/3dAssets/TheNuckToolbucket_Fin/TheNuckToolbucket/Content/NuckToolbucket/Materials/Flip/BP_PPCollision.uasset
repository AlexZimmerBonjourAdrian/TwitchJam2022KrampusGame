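; Trigger volume that flips the screen through a post-process material while the player character is inside its box.
; BeginPlay creates a dynamic instance of MI_Flip and adds it to the PPFlip post-process component as a blendable, initially disabled.
; Box overlaps play forward and reverse timelines that drive the flip scale parameter, disabling the post process once the exit animation finishes.
; An unconnected FlipPlayerMessage call relates to flipping both axes with BP_NuckManFlipped.
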(event OnComponentBeginOverlap(Box)
  (params (OverlappedComponent :type Primitive%20Component%20Object%20Reference) (OtherActor :type Actor%20Object%20Reference) (OtherComp :type Primitive%20Component%20Object%20Reference) (OtherBodyIndex :type Integer) (bFromSweep :type Boolean) (SweepResult :type Hit%20Result%20Structure%20%28by%20ref%29))
  (Utilities|IsPlayer OtherActor
    (:Yes
      (Variables|/Script/Engine.PostProcessComponent|SetbEnabled (Variables|Default|GetPPFlip) true)
      (Components|Timeline|SetPlayRate (Variables|Default|GetFlipLerp) (Variables|Default|GetFlipRateMultiplier))
      (bind _amount (Timeline|FlipLerp PlayFromStart)
        (:Update
          (Rendering|Material|SetScalarParameterValue (Variables|Default|GetFlipMatRef) (Variables|Default|GetFlipScaleName) _amount :!class /Script/Engine.MaterialInstanceDynamic))))))

(event OnComponentEndOverlap(Box)
  (params (OverlappedComponent :type Primitive%20Component%20Object%20Reference) (OtherActor :type Actor%20Object%20Reference) (OtherComp :type Primitive%20Component%20Object%20Reference) (OtherBodyIndex :type Integer))
  (Utilities|IsPlayer OtherActor
    (:Yes
      (Components|Timeline|SetPlayRate (Variables|Default|GetReverseFlipLerp) (Variables|Default|GetFlipRateMultiplier))
      (bind _amount (Timeline|ReverseFlipLerp PlayFromStart)
        (:Update
          (Rendering|Material|SetScalarParameterValue (Variables|Default|GetFlipMatRef) (Variables|Default|GetFlipScaleName) _amount :!class /Script/Engine.MaterialInstanceDynamic))
        (:Finished
          (Variables|/Script/Engine.PostProcessComponent|SetbEnabled (Variables|Default|GetPPFlip) false))))))

(event EventBeginPlay
  (bind _returnvalue (Rendering|Material|CreateDynamicMaterialInstance "/Game/NuckToolbucket/Materials/Flip/MI_Flip.MI_Flip" "None" :!class /Script/Engine.KismetMaterialLibrary))
  (bind _output_get (Variables|Default|SetFlipMatRef _returnvalue))
  (Variables|/Script/Engine.PostProcessComponent|SetSettings (Variables|Default|GetPPFlip) (Utilities|Struct|MakePostProcessSettings (Utilities|Struct|MakeWeightedBlendables (Utilities|Array|MakeArray (Utilities|Struct|MakeWeightedBlendable 1.0 _output_get)))))
  (Rendering|Material|SetScalarParameterValue (Variables|Default|GetFlipMatRef) (Variables|Default|GetFlipScaleName) 0.0 :!class /Script/Engine.MaterialInstanceDynamic)
  (Variables|/Script/Engine.PostProcessComponent|SetbEnabled (Variables|Default|GetPPFlip) false))

(fn ConstructionScript)