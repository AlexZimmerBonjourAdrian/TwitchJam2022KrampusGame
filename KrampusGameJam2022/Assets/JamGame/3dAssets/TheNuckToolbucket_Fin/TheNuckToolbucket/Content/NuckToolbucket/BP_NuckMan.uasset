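; BP_NuckMan is a Blueprint with a CameraBoom that lets the player zoom the camera in and out.
; Pressing the ZoomIn or ZoomOut input action subtracts or adds ZoomRate to the boom's TargetArmLength.
; Each press applies one immediate step, with no clamping or interpolation in the graph, and the construction script is empty.
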(event Input|ActionEvents|InputActionZoomIn
  (params (Key :type Key%20Structure))
  (:Pressed
    (Variables|/Script/Engine.SpringArmComponent|SetTargetArmLength (Variables|Default|GetCameraBoom) (- (Variables|/Script/Engine.SpringArmComponent|GetTargetArmLength (Variables|Default|GetCameraBoom)) (Variables|Default|GetZoomRate)))))

(event Input|ActionEvents|InputActionZoomOut
  (params (Key :type Key%20Structure))
  (:Pressed
    (Variables|/Script/Engine.SpringArmComponent|SetTargetArmLength (Variables|Default|GetCameraBoom) (+ (Variables|Default|GetZoomRate) (Variables|/Script/Engine.SpringArmComponent|GetTargetArmLength (Variables|Default|GetCameraBoom))))))

(fn ConstructionScript)