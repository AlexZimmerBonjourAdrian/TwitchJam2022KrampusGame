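; BP_DynamicColourChanger is an actor that continuously cycles the colour of a static mesh and its point light together.
; On BeginPlay it creates a dynamic instance of MI_ColourChanger and applies a shared intensity to the material and, scaled by a multiplier, the light.
; A timeline with adjustable speed drives both colours, restarting after a zero-length delay whenever it finishes to loop endlessly.
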(event Custom|LoopColour
  (Components|Timeline|SetPlayRate (Variables|Default|GetColourChanger) (Variables|Default|GetColourChangeSpeed))
  (bind _colourvalue (Timeline|ColourChanger PlayFromStart)
    (:Update
      (Rendering|Material|SetVectorParameterValue (Variables|Default|GetMaterialRef) "Colour" (Math|Conversions|ToLinearColor(Vector) _colourvalue) :!class /Script/Engine.MaterialInstanceDynamic)
      (Rendering|Components|Light|SetLightColor (Variables|Default|GetPointLight) (Math|Conversions|ToLinearColor(Vector) _colourvalue) true))
    (:Finished
      (Utilities|FlowControl|Delay 0.0)
      (Timeline|ColourChanger PlayFromStart))))

(event EventBeginPlay
  (bind _returnvalue (Rendering|Material|CreateDynamicMaterialInstance (Variables|Default|GetStaticMesh) 0 "/Game/NuckToolbucket/Materials/ColourChanger/MI_ColourChanger.MI_ColourChanger" "None" :!class /Script/Engine.PrimitiveComponent))
  (bind _output_get (Variables|Default|SetMaterialRef _returnvalue))
  (Rendering|Material|SetScalarParameterValue _output_get "Intensity" (Variables|Default|GetIntensity) :!class /Script/Engine.MaterialInstanceDynamic)
  (Rendering|Components|Light|SetIntensity (Variables|Default|GetPointLight) (* (Variables|Default|GetIntensity) (Variables|Default|GetLightIntensityMultiplier)))
  (CallFunction|LoopColour))

(fn ConstructionScript)