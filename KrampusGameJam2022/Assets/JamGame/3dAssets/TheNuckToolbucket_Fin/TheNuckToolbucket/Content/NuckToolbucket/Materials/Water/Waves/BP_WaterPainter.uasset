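; Water volume actor that paints ripples under actors inside its collision box, with a scene capture that renders only this actor.
; A pool of five ripple particle systems is assigned on overlap, including actors present at BeginPlay, and released shortly after exit.
; Tick pins assigned ripples to the water surface at each actor's XY and raises spawn rate above a speed threshold.
; Timeline-driven bobbing logic exists but is disconnected.
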(event OnComponentBeginOverlap(WaterCollision)
  (params (OverlappedComponent :type Primitive%20Component%20Object%20Reference) (OtherActor :type Actor%20Object%20Reference) (OtherComp :type Primitive%20Component%20Object%20Reference) (OtherBodyIndex :type Integer) (bFromSweep :type Boolean) (SweepResult :type Hit%20Result%20Structure%20%28by%20ref%29))
  (bind (_array_element _array_index) (Utilities|Array|ForEachLoopwithBreak (Variables|Default|GetParticleSystemPool) :!label _label)
    (:LoopBody
      (if (not (.IsAssigned (Utilities|Struct|BreakS_WaveInfo _array_element)))
        (Utilities|Array|SetArrayElem (Variables|Default|GetParticleSystemPool) _array_index (Utilities|Struct|MakeS_WaveInfo (.ParticleSystem (Utilities|Struct|BreakS_WaveInfo _array_element)) OtherActor true))
        (goto _label Break)))))

(event OnComponentEndOverlap(WaterCollision)
  (params (OverlappedComponent :type Primitive%20Component%20Object%20Reference) (OtherActor :type Actor%20Object%20Reference) (OtherComp :type Primitive%20Component%20Object%20Reference) (OtherBodyIndex :type Integer))
  (bind (_array_element _array_index) (Utilities|Array|ForEachLoopwithBreak (Variables|Default|GetParticleSystemPool) :!label _label)
    (:LoopBody
      (if (== (.OverlapActor (Utilities|Struct|BreakS_WaveInfo _array_element)) OtherActor)
        (Utilities|FlowControl|Delay 0.2)
        (Utilities|Array|SetArrayElem (Variables|Default|GetParticleSystemPool) _array_index (Utilities|Struct|MakeS_WaveInfo (.ParticleSystem (Utilities|Struct|BreakS_WaveInfo _array_element)) 0 false))
        (goto _label Break)))))

(event Custom|CheckFloatMovement
  (params (Collider :type Actor%20Object%20Reference) (StartFloating :type Boolean))
  (if (< (.Z (Math|Vector|BreakVector (.BoxExtent (Collision|GetActorBounds Collider false)))) (* (.Z (Math|Vector|BreakVector (.BoxExtent (Collision|GetComponentBounds (Variables|Default|GetWaterCollision))))) 2.0))
    (CallFunction|StartFloating Collider)))

(event Custom|AddParticleSystems
  (Variables|Default|SetCurrentSystems (Utilities|Array|MakeArray (Variables|Default|GetRipples0) (Variables|Default|GetRipples1))))

(event Custom|StartFloating
  (params (ActorRef :type Actor%20Object%20Reference))
  (bind _returnvalue (Transformation|GetActorLocation ActorRef))
  (Components|Timeline|SetPlayRate (Variables|Default|GetFloating) (Variables|Default|GetFloatSpeed))
  (bind _floatmultiplier (Timeline|Floating PlayFromStart)
    (:Update
      (Transformation|SetActorLocation ActorRef (Math|Vector|MakeVector (.x _returnvalue) (.y _returnvalue) (+ (* (- _floatmultiplier (Variables|Default|GetLastTime)) (Variables|Default|GetMaxOffset) (Variables|Default|GetFloatSpeed)) (.z _returnvalue))) false false)
      (Variables|Default|SetLastTime _floatmultiplier))
    (:Finished
      (Variables|Default|SetMaxOffset (Variables|Default|GetMaxOffset))
      (Timeline|Floating PlayFromStart))))

(event Custom|CreatePool
  (Utilities|Array|Clear (Variables|Default|GetParticleSystemPool))
  (for _array_element (Utilities|Array|MakeArray (Variables|Default|GetRipples0) (Variables|Default|GetRipples1) (Variables|Default|GetRipples2) (Variables|Default|GetRipples3) (Variables|Default|GetRipples4))
    (Utilities|Array|AddUnique (Variables|Default|GetParticleSystemPool) (Utilities|Struct|MakeS_WaveInfo _array_element 0 false))))

(event Custom|SetupStartOverlaps
  (bind (_array_element _array_index) (Utilities|Array|ForEachLoopwithBreak (Collision|GetOverlappingActors (Variables|Default|GetWaterCollision) 0 :!class /Script/Engine.PrimitiveComponent) :!label _label)
    (:LoopBody
      (if (< _array_index (Utilities|Array|Length (Variables|Default|GetParticleSystemPool)))
        (bind (_array_element_2 _array_index_2) (Utilities|Array|ForEachLoopwithBreak (Variables|Default|GetParticleSystemPool) :!label _label_2)
          (:LoopBody
            (if (not (.IsAssigned (Utilities|Struct|BreakS_WaveInfo _array_element_2)))
              (Utilities|Array|SetArrayElem (Variables|Default|GetParticleSystemPool) _array_index_2 (Utilities|Struct|MakeS_WaveInfo (.ParticleSystem (Utilities|Struct|BreakS_WaveInfo _array_element_2)) _array_element true))
              (goto _label_2 Break))))
        (else
          (goto _label Break))))))

(event Custom|StopFloating
  (Variables|Default|SetLastTime 0.0)
  (bind _floatmultiplier (Timeline|Floating Stop)
    (:Update
      (Transformation|SetActorLocation (stale Custom|StartFloating ActorRef) (Math|Vector|MakeVector (.x (Transformation|GetActorLocation (stale Custom|StartFloating ActorRef))) (.y (Transformation|GetActorLocation (stale Custom|StartFloating ActorRef))) (+ (* (- _floatmultiplier (Variables|Default|GetLastTime)) (Variables|Default|GetMaxOffset) (Variables|Default|GetFloatSpeed)) (.z (Transformation|GetActorLocation (stale Custom|StartFloating ActorRef))))) false false)
      (Variables|Default|SetLastTime _floatmultiplier))
    (:Finished
      (Variables|Default|SetMaxOffset (Variables|Default|GetMaxOffset))
      (Timeline|Floating PlayFromStart))))

(event EventTick
  (params (DeltaSeconds :type Float%20%28single-precision%29))
  (bind _watercollision (Variables|Default|GetWaterCollision))
  (if (> (Utilities|Array|Length (Variables|Default|GetParticleSystemPool)) 0)
    (for _array_element (Variables|Default|GetParticleSystemPool)
      (if (.IsAssigned (Utilities|Struct|BreakS_WaveInfo _array_element))
        (Rendering|SetVisibility (.ParticleSystem (Utilities|Struct|BreakS_WaveInfo _array_element)) true false)
        (Transformation|SetWorldLocation (.ParticleSystem (Utilities|Struct|BreakS_WaveInfo _array_element)) (Math|Vector|MakeVector (.X (Math|Vector|BreakVector (Transformation|GetActorLocation (.OverlapActor (Utilities|Struct|BreakS_WaveInfo _array_element))))) (.Y (Math|Vector|BreakVector (Transformation|GetActorLocation (.OverlapActor (Utilities|Struct|BreakS_WaveInfo _array_element))))) (+ (.z (Transformation|GetWorldLocation _watercollision)) (.z (Components|Box|GetScaledBoxExtent _watercollision)))) true false)
        (if (> (Math|Vector|VectorLengthSquared (Transformation|GetVelocity (.OverlapActor (Utilities|Struct|BreakS_WaveInfo _array_element)))) (Variables|Default|GetLowestSpeed))
          (Effects|Components|ParticleSystem|SetFloatParameter (.ParticleSystem (Utilities|Struct|BreakS_WaveInfo _array_element)) "SpawnRate" 15.0)
          (else
            (Effects|Components|ParticleSystem|SetFloatParameter (.ParticleSystem (Utilities|Struct|BreakS_WaveInfo _array_element)) "SpawnRate" 2.0)))
        (else
          (Rendering|SetVisibility (.ParticleSystem (Utilities|Struct|BreakS_WaveInfo _array_element)) false false))))))

(event EventBeginPlay
  (Actor|SetOwner (Game|GetPlayerCharacter 0))
  (Variables|/Script/Engine.SceneCaptureComponent|SetShowOnlyActors (Variables|Default|GetSceneCaptureComponent2D) (Utilities|Array|MakeArray self))
  (CallFunction|CreatePool)
  (CallFunction|SetupStartOverlaps))

(fn ConstructionScript)